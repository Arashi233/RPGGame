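; BP_ManaPotion is a pickup actor that applies an instant gameplay effect to the actor that overlaps it.
; Its Sphere overlap passes InstantGameplayEffectClass to ApplyEffectToTarget, then destroys the potion without filtering the other actor.
; Each Tick spins it in yaw by delta time and adds a game-time sine offset to its current Z, so the bobbing depends on frame rate.
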(event OnComponentBeginOverlap(Sphere)
  (params (OverlappedComponent :type Primitive%20Component%20Object%20Reference) (OtherActor :type Actor%20Object%20Reference) (OtherComp :type Primitive%20Component%20Object%20Reference) (OtherBodyIndex :type Integer) (bFromSweep :type Boolean) (SweepResult :type Hit%20Result%20Structure%20%28by%20ref%29))
  (Class|AuraEffectActor|ApplyEffecttoTarget OtherActor (Variables|Default|GetInstantGameplayEffectClass))
  (Actor|DestroyActor))

(event EventBeginPlay)

(event Collision|EventActorBeginOverlap
  (params (OtherActor :type Actor%20Object%20Reference)))

(event EventTick
  (params (DeltaSeconds :type Float%20%28single-precision%29))
  (CallFunction|UpdateFloatingandRotation DeltaSeconds))

(fn ConstructionScript)

(fn UpdateFloatingandRotation
  (params (A :type Float%20%28double-precision%29))
  (bind _returnvalue (Transformation|GetActorLocation))
  (Transformation|AddActorLocalRotation (Math|Rotator|MakeRotator 0.0 0.0 (* A 5e+01)) false false)
  (Transformation|SetActorLocation (Math|Vector|MakeVector (.x _returnvalue) (.y _returnvalue) (+ (.z _returnvalue) (* (Math|Trig|Sin(Radians) (* (Utilities|Time|GetGameTimeinSeconds) (Variables|Default|GetSpeed))) (Variables|Default|GetAmplitude)))) false false))